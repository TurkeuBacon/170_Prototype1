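; Player bow that is drawn by holding left mouse and spawns a Box at FirePos on release.
; Drawing locks the first-person character's camera and accumulates mouse travel into a draw strength with diminishing returns toward MaxDrawPower; right mouse temporarily restores look and pauses the draw.
; Tick scrubs the bow animation to match draw strength, then plays out the release from the mirrored position.
; Draw strength is not applied to the spawned Box here.
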(event `self.ReceiveBeginPlay`
  (bind _asbp_first_person_character (cast `/Game/FirstPerson/Blueprints/BP_FirstPersonCharacter` (`GameplayStatics.GetPlayerCharacter` 0)))
  (set `self.PlayerRef` _asbp_first_person_character))

(event `fire`
  (`|SpawnActorFromClass` "/Game/box.box_C" (`SceneComponent.K2_GetComponentToWorld` (`self.firePos`)) "AlwaysSpawn" "MultiplyWithRoot" null null))

(event `self.ReceiveTick`
  (params (DeltaSeconds :type "Float (single-precision)"))
  (`self.UpdateDrawnStrength` DeltaSeconds)
  (`self.UpdateBowAnimation`))

(event `Key|LeftMouseButton`
  (params (Key :type "Key Structure"))
  (bind _playerref (`self.PlayerRef`))
  (:`Pressed`
    (set `self.DrawingBow` true)
    (`/Game/FirstPerson/Blueprints/BP_FirstPersonCharacter.lockCameraAxisY` _playerref)
    (`/Game/FirstPerson/Blueprints/BP_FirstPersonCharacter.lockCameraAxisX` _playerref)
    (set `self.BowAnimSetpoint` 0.0 :!label _label)
    (set `self.DrawMouseTravel` 0.0)
    (set `self.DrawStrength` 0.0))
  (:`Released`
    (set `self.DrawingBow` false)
    (`/Game/FirstPerson/Blueprints/BP_FirstPersonCharacter.unlockCameraAxisY` _playerref)
    (`/Game/FirstPerson/Blueprints/BP_FirstPersonCharacter.unlockCameraAxisX` _playerref)
    (`self.fire`)
    (goto _label)))

(event `Key|RightMouseButton`
  (params (Key :type "Key Structure"))
  (bind _playerref (`self.PlayerRef`))
  (:`Pressed`
    (set `self.DrawLook` true)
    (`/Game/FirstPerson/Blueprints/BP_FirstPersonCharacter.unlockCameraAxisY` _playerref)
    (`/Game/FirstPerson/Blueprints/BP_FirstPersonCharacter.unlockCameraAxisX` _playerref))
  (:`Released`
    (set `self.DrawLook` false)
    (if (`self.DrawingBow`)
      (`/Game/FirstPerson/Blueprints/BP_FirstPersonCharacter.lockCameraAxisY` _playerref)
      (`/Game/FirstPerson/Blueprints/BP_FirstPersonCharacter.lockCameraAxisX` _playerref))))

(fn `Try Fire`
  (returns (Success :type Boolean))
  (`self.fire`)
  (return true))

(fn `UpdateBowAnimation`
  (bind _bow (`self.bow`))
  (bind _returnvalue (`SkeletalMeshComponent.GetPosition` _bow))
  (if (`self.DrawingBow`)
    (if (`SkeletalMeshComponent.IsPlaying` _bow)
      (`SkeletalMeshComponent.SetPosition` _bow (`self.BowAnimSetpoint`) true)
      (else
        (`SkeletalMeshComponent.PlayAnimation` _bow "/Game/Assets/Bow/SK_CupidBow01_Anim_BowBones_BowBonesAction.SK_CupidBow01_Anim_BowBones_BowBonesAction" false)))
    (elif (< _returnvalue 0.5)
      (`SkeletalMeshComponent.SetPosition` _bow (- 1.0 _returnvalue) true)
      (`SkeletalMeshComponent.SetPlayRate` _bow 1.0))))

(fn `UpdateDrawnStrength`
  (params (dt :type "Float (double-precision)"))
  (bind _maxdrawpower (`self.maxDrawPower`))
  (if (and (not (`self.DrawLook`)) (`self.DrawingBow`))
    (bind _output_get (set `self.DrawMouseTravel` (`KismetMathLibrary.FClamp` (+ (* dt (`self.GetInputAxisKeyValue`) -50.0) (`self.DrawMouseTravel`)) 0.0 1000.0)))
    (bind _output_get_2 (set `self.DrawStrength` (+ (* (`KismetMathLibrary.MultiplyMultiply_FloatFloat` (+ (/ _output_get (`self.stretch`)) (`KismetMathLibrary.MultiplyMultiply_FloatFloat` _maxdrawpower -1.0)) -1.0) -1.0) _maxdrawpower)))
    (set `self.BowAnimSetpoint` (/ _output_get_2 (`self.maxDrawPower`) 2.0))))

(fn `UserConstructionScript`)