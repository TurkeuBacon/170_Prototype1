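; Arrow projectile actor that turns its SKHeartArrow01 component to follow its flight.
; Every Tick, GetRotation scales the normalized ArrowMovement velocity by 180, adds a -90 offset on Z, and feeds the result into the relative rotation as roll, yaw and pitch from X, Y and Z.
; This is a linear approximation rather than a true direction-to-rotation conversion; an arctangent variant and a world-rotation call are left unused.
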(event `self.ReceiveTick`
  (params (DeltaSeconds :type "Float (single-precision)"))
  (bind _rotation (`self.getRotation`))
  (`SceneComponent.K2_SetRelativeRotation` (`self.SK_HeartArrow01`) (`KismetMathLibrary.MakeRotator` (.x _rotation) (.z _rotation) (.y _rotation)) false false)
  (`SceneComponent.K2_SetRelativeRotation` (`self.SK_HeartArrow01`) (`KismetMathLibrary.MakeRotator` (.x _rotation) (.z _rotation) (.y _rotation)) false false))

(fn `getRotation`
  (returns (rotation :type "Vector Structure"))
  (return (+ (* (`KismetMathLibrary.Normal` (`MovementComponent.Velocity` (`self.ArrowMovement`))) 180.0) (0.0 0.0 -90.0))))

(fn `UserConstructionScript`)