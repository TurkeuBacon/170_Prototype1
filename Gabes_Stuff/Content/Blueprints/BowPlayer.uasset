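; Player Blueprint for bow aiming that previews a projectile arc while the left mouse button is held; no arrow is fired here.
; Input axes turn the actor and pitch the camera, but while drawing they adjust draw strength instead of pitch unless right mouse is held.
; Draw strength sets velocity through a power curve.
; Each tick five points are chained along an analytic parabola, using slope-corrected steps for even arc-length spacing.
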(event `self.ReceiveBeginPlay`
  (`self.SetPlayerStart`)
  (`self.setupPointsList`))

(event `self.ReceiveTick`
  (params (DeltaSeconds :type "Float (single-precision)"))
  (`self.SetPlayerRotation` DeltaSeconds)
  (`self.UpdateVelocity` DeltaSeconds)
  (`self.updatePoints`))

(event `Key|LeftMouseButton`
  (params (Key :type "Key Structure"))
  (:`Pressed`
    (set `self.drawingBow` true)
    (set `self.drawStrength` 0.0 :!label _label)
    (set `self.velocity` 0.0)
    (for _array_element (`self.pointsList`)
      (`SceneComponent.SetVisibility` _array_element (`self.drawingBow`) false)))
  (:`Released`
    (set `self.drawingBow` false)
    (goto _label)))

(event `Key|RightMouseButton`
  (params (Key :type "Key Structure"))
  (:`Pressed`
    (set `self.drawLook` true))
  (:`Released`
    (set `self.drawLook` false)))

(fn `Parabola`
  (params (x :type "Float (double-precision)") (velocity :type "Float (double-precision)") (angle :type "Float (double-precision)") (g :type "Float (double-precision)"))
  (returns (z :type "Float (double-precision)"))
  (bind _returnvalue (`KismetMathLibrary.DegCos` angle))
  (return (- (* x (`KismetMathLibrary.DegTan` angle)) (* x x (/ g (* velocity velocity _returnvalue _returnvalue 2.0))))))

(fn `SetPlayerRotation`
  (params (dt :type "Float (double-precision)"))
  (bind _output_get (set `self.Rotation` (+ (* dt (`self.rotSpeed`) (`KismetMathLibrary.MakeVector` 0.0 (select `bool` (or (not (`self.drawingBow`)) (`self.drawLook`)) :`true` (`self.GetInputAxisKeyValue`)) (`self.GetInputAxisKeyValue`))) (`self.Rotation`))))
  (`self.K2_SetActorRotation` (`KismetMathLibrary.MakeRotator` 0.0 0.0 (.z _output_get)))
  (`SceneComponent.K2_SetRelativeRotation` (`self.Camera`) (`KismetMathLibrary.MakeRotator` 0.0 (.y _output_get)) false false))

(fn `SetPlayerStart`
  (set `self.Rotation` (`KismetMathLibrary.Conv_RotatorToVector` (`self.K2_GetActorRotation`)))
  (`self.K2_SetActorLocation` (`KismetMathLibrary.MakeVector` 0.0 0.0 100.0)))

(fn `setupPointsList`
  (set `self.pointsList` (`|MakeArray` (`self.p1`) (`self.p2`) (`self.p3`) (`self.p4`) (`self.p5`))))

(fn `Step`
  (params (x :type "Float (double-precision)") (angle :type "Float (double-precision)") (velocity :type "Float (double-precision)") (g :type "Float (double-precision)") (m :type "Float (double-precision)"))
  (returns (step :type "Float (double-precision)"))
  (bind _returnvalue (`KismetMathLibrary.DegCos` angle))
  (bind _returnvalue_2 (- (`KismetMathLibrary.DegTan` angle) (* x (/ g (* velocity velocity _returnvalue _returnvalue)))))
  (return (/ m (`KismetMathLibrary.Sqrt` (+ (* _returnvalue_2 _returnvalue_2) 1.0)))))

(fn `updatePoints`
  (bind _velocity (`self.velocity`))
  (bind _pointslist (`self.pointsList`))
  (bind _y (.y (`self.Rotation`)))
  (for (_array_element _array_index) _pointslist
    (bind _returnvalue (> _array_index 0))
    (bind _x (.x (`KismetMathLibrary.SelectVector` (`SceneComponent.RelativeLocation` (`|GetArrayItem` _pointslist (`KismetMathLibrary.SelectInt` (- _array_index 1) 0 _returnvalue))) (0.0 0.0 0.0) _returnvalue)))
    (bind _step (`self.Step` _x _y _velocity 9.8 (* _velocity _velocity 0.005)))
    (bind _returnvalue_2 (+ _x _step))
    (bind _z (`self.Parabola` _returnvalue_2 _velocity _y 9.8))
    (`SceneComponent.K2_SetRelativeLocation` _array_element (+ (`SceneComponent.RelativeLocation` (`self.Camera`)) (`KismetMathLibrary.MakeVector` _returnvalue_2 0.0 _z) (0.0 25.0 -25.0)) false false)))

(fn `UpdateVelocity`
  (params (dt :type "Float (double-precision)"))
  (bind _returnvalue (`self.GetInputAxisKeyValue`))
  (if (and (not (`self.drawLook`)) (`self.drawingBow`))
    (bind _output_get (set `self.drawStrength` (`KismetMathLibrary.FClamp` (+ (* dt _returnvalue -50.0) (`self.drawStrength`)) 0.0 1000.0)))
    (set `self.velocity` (* 100.0 (`KismetMathLibrary.MultiplyMultiply_FloatFloat` _output_get 0.2)))
    (`KismetSystemLibrary.PrintString` (`KismetStringLibrary.Conv_DoubleToString` _returnvalue))))

(fn `UserConstructionScript`)