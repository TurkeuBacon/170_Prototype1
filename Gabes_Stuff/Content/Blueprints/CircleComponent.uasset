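; CircleComponent is an actor component that bobs its owning actor up and down, despite its name.
; Each Tick keeps the owner's X and Y and sets Z from a sine of game time, oscillating between StartHeight and StartHeight plus Amplitude.
; The move skips sweeping, the speed is not adjustable, and StartHeight is never assigned in this graph.
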(event `self.ReceiveTick`
  (params (DeltaSeconds :type "Float (single-precision)"))
  (bind _returnvalue (`self.GetOwner`))
  (bind _returnvalue_2 (/ (`self.Amplitude`) 2.0))
  (`Actor.K2_SetActorLocation` _returnvalue (`KismetMathLibrary.MakeVector` (.x (`Actor.K2_GetActorLocation` _returnvalue)) (.y (`Actor.K2_GetActorLocation` _returnvalue)) (+ (* (`KismetMathLibrary.Sin` (`GameplayStatics.GetTimeSeconds`)) _returnvalue_2) (`self.StartHeight`) _returnvalue_2)) false false))